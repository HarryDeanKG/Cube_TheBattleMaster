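; Projectile path preview module that shows the predicted trajectory of the selected item from the mouse position and the item's facing.
; When activated, a looping timer reruns the path prediction about 60 times a second until deactivation hides it.
; Path points become oriented instanced meshes, reusing instances, zero-scaling extras and dirtying render state once per update.
; An optional decal marks the blocking hit, aligned to its surface normal.
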(event Custom|ActivateModule
  (bind _returnvalue (Utilities|Time|SetTimerbyEvent (delegate Custom|DisplayTrajectory) 0.016667 true)) ; Starts timer to calculate & display predicted projectile path repeatedly
  (Variables|TimerHandles|SetPathDisplayTimer _returnvalue))

(event Custom|DeactivateModule
  (Utilities|Time|ClearandInvalidateTimerbyHandle (Variables|TimerHandles|GetPathDisplayTimer))
  (CallFunction|HideTrajectory))

(event Custom|HideTrajectory
  (Components|InstancedStaticMesh|ClearInstances (Variables|Default|GetProjectilePathMesh))
  (Development|SetHiddeninGame (Variables|Default|GetDecal) true false))

(event Custom|DisplayTrajectory
  (bind _returnvalue (Game|GetPlayerController 0))
  (bind _itemselected (Variables|Default|GetItemSelected))
  (bind _projectilepathmesh (Variables|Default|GetProjectilePathMesh))
  (bind _projectilepathmesh_2 (Variables|Default|GetProjectilePathMesh))
  (bind _projectilepathmesh_3 (Variables|Default|GetProjectilePathMesh))
  (bind _decal (Variables|Default|GetDecal))
  (bind _returnvalue_2 (Transformation|GetActorForwardVector _itemselected))
  (bind _returnvalue_3 (Components|InstancedStaticMesh|GetInstanceCount _projectilepathmesh))
  (bind _returnvalue_4 (Transformation|GetActorLocation _itemselected))
  (bind (_worldlocation _worlddirection) (Game|Player|ConvertMouseLocationToWorldSpace _returnvalue))
  (bind _returnvalue_5 (Components|InstancedStaticMesh|GetInstanceCount _projectilepathmesh_2))
  (bind _returnvalue_6 (* _returnvalue_2 15.0))
  (bind _returnvalue_7 (- _returnvalue_5 1))
  (bind (_outhit _outpathpositions _outlasttracedestination _returnvalue_8) (Class|GameplayStatics|BlueprintPredictProjectilePathbyTraceChannel (+ _returnvalue_4 _returnvalue_6) (* (+ _returnvalue_6 _worlddirection) (/ (Math|Vector|Distance(Vector) _worldlocation (+ _returnvalue_4 (* _worlddirection (/ (- 1e+02 (.Z (Math|Vector|BreakVector _returnvalue_4))) (.Z (Math|Vector|BreakVector _worlddirection)))))) 1e+01)) true 0.1 "ECC_Visibility" true (Utilities|Array|MakeArray _itemselected 0) "None" 0.0 1e+03))
  ;[0 1 1 0.5] Uses instanced static mesh component to represent all predicted path points in world space
  (Development|PrintString (Utilities|String|ToString(Boolean) _returnvalue_8))
  (for _index (range 0 (- (Utilities|Array|Length _outpathpositions) 2)) ; Loops through all path points excluding the final one
    (if (< (+ _index 1) (Components|InstancedStaticMesh|GetInstanceCount (Variables|Default|GetProjectilePathMesh))) ; Checks if there are enough instances
      (Components|InstancedStaticMesh|UpdateInstanceTransform _projectilepathmesh_3 _index (Math|Transform|MakeTransform (Utilities|Array|Get(acopy) _outpathpositions _index) (Math|Rotator|MakeRotator (.Roll (Math|Rotator|BreakRotator (Math|Conversions|RotationFromXVector (- (Utilities|Array|Get(acopy) _outpathpositions (+ _index 1)) (Utilities|Array|Get(acopy) _outpathpositions _index))))) (+ (.Pitch (Math|Rotator|BreakRotator (Math|Conversions|RotationFromXVector (- (Utilities|Array|Get(acopy) _outpathpositions (+ _index 1)) (Utilities|Array|Get(acopy) _outpathpositions _index))))) 9e+01) (.Yaw (Math|Rotator|BreakRotator (Math|Conversions|RotationFromXVector (- (Utilities|Array|Get(acopy) _outpathpositions (+ _index 1)) (Utilities|Array|Get(acopy) _outpathpositions _index))))))) true false true) ; Uses an existing mesh instance to display the path point
      (else
        (Class|InstancedStaticMeshComponent|AddInstanceWorldSpace _projectilepathmesh_3 (Math|Transform|MakeTransform (Utilities|Array|Get(acopy) _outpathpositions _index) (Math|Rotator|MakeRotator (.Roll (Math|Rotator|BreakRotator (Math|Conversions|RotationFromXVector (- (Utilities|Array|Get(acopy) _outpathpositions (+ _index 1)) (Utilities|Array|Get(acopy) _outpathpositions _index))))) (+ (.Pitch (Math|Rotator|BreakRotator (Math|Conversions|RotationFromXVector (- (Utilities|Array|Get(acopy) _outpathpositions (+ _index 1)) (Utilities|Array|Get(acopy) _outpathpositions _index))))) 9e+01) (.Yaw (Math|Rotator|BreakRotator (Math|Conversions|RotationFromXVector (- (Utilities|Array|Get(acopy) _outpathpositions (+ _index 1)) (Utilities|Array|Get(acopy) _outpathpositions _index)))))))) ; Creates a new mesh instance to display the path point
        (Development|PrintString (Utilities|String|ToString(Vector) (Utilities|Array|Get(acopy) _outpathpositions _index))))))
  ;[0 1 1 0.5] Scales down any unused mesh instances to make them invisible
  (if (< (- (Utilities|Array|Length _outpathpositions) 1) _returnvalue_3) ; Checks if there are extra unused mesh instances
    (for _index_2 (range (- (Utilities|Array|Length _outpathpositions) 1) (- _returnvalue_3 1))
      (Components|InstancedStaticMesh|UpdateInstanceTransform (Variables|Default|GetProjectilePathMesh) _index_2 (Math|Transform|MakeTransform "0, 0, 0" "0, 0, 0" "0.000000,0.000000,0.000000") true false true) ; Scaled down to zero to make the instance invisible
    ))
  ;[0 1 1 0.5] Forces the transform updates to happen immediately
  (Components|InstancedStaticMesh|UpdateInstanceTransform (Variables|Default|GetProjectilePathMesh) _returnvalue_7 (.OutInstanceTransform (Components|InstancedStaticMesh|GetInstanceTransform (Variables|Default|GetProjectilePathMesh) _returnvalue_7 true)) true true true) ; "Make Render State Dirty" applied to last mesh instance to force immediate transform updates
  ;[0 1 1 0.5] Displays impact marker at the predicted hit location
  (if (Variables|Config|GetDisplayImpactMarker?)
    (if (.bBlockingHit (Collision|BreakHitResult _outhit))
      (Transformation|SetWorldTransform (Variables|Default|GetDecal) (Math|Transform|MakeTransform (.ImpactPoint (Collision|BreakHitResult _outhit)) (Math|Conversions|RotationFromXVector (.ImpactNormal (Collision|BreakHitResult _outhit)))) false false)
      (Development|SetHiddeninGame _decal false false)
      (else
        (Development|SetHiddeninGame _decal true false)))))

(fn ConstructionScript)