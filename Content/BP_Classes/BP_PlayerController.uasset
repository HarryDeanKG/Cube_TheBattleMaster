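; Player controller that sets up each player's pawn and handles the hand-off from UI to gameplay.
; On BeginPlay it derives a player number from the controller count on the server, possesses a BP_Pawn spawned at the PlayerStart with that index, and enters UI-only input.
; Server_FlagReadyToPlay tells BP_TheBattleMasterGameMode to begin the game.
; SetReadytoPlay clears widgets and switches to game-and-UI input.
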(event Custom|Server_FlagReadyToPlay
  (CallFunction|ReadytoPlay))

(event EventBeginPlay
  (CallFunction|AssignPlayerNumber)
  (CallFunction|MakePawn)
  (Input|SetInputModeUIOnly self 0 "DoNotLock"))

(event EventTick
  (params (DeltaSeconds :type Float%20%28single-precision%29)))

(event EventSetReadytoPlay
  (Viewport|RemoveAllWidgets)
  (Input|SetInputModeGameandUI self 0 "DoNotLock" true))

(fn ConstructionScript)

(fn AssignPlayerNumber
  (if (Networking|IsServer)
    (bind _outactors (Actor|GetAllActorsOfClass "BP_PlayerController_C"))
    (if (== (Utilities|Array|Length _outactors) 0)
      (Variables|Default|SetPlayerNumb 0)
      (else
        (Variables|Default|SetPlayerNumb (+ (Utilities|Array|LastIndex _outactors) 1))))))

(fn MakePawn
  (bind _outactors (Actor|GetAllActorsOfClass "/Script/Engine.PlayerStart"))
  (bind (_array_element _array_index) (Utilities|Array|ForEachLoopwithBreak _outactors)
    (:LoopBody
      (if (== (Variables|Default|GetPlayerNumb) _array_index)
        (bind _returnvalue (Game|SpawnActorfromClass "/Game/BP_Classes/BP_Pawn.BP_Pawn_C" (Transformation|GetActorTransform _array_element) "Undefined" self 0))
        (Pawn|Possess _returnvalue)))))

(fn ReadytoPlay
  (Class|CubetheBattleMasterGameMode|BegintheGame (.AsBP%20the%20Battle%20Master%20Game%20Mode (Utilities|Casting|CastToBP_TheBattleMasterGameMode (Game|GetGameMode)))))