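; Player pawn for a turn-based cube combat game, linking action-planning events to the player's UI and handling cube setup.
; Local players get character selection, waiting, action and ammo/energy widgets, with buttons toggled on confirm, cancel and ready.
; Server and multicast events share cube class, material and save data; MakeCube spawns the cube and binds its attachment inventory to an equip widget.
; Includes camera cycling, temporary random item attachment and debug key hooks.
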(event Custom|MakeCube
  (CallFunction|TogglleCamera)
  (if (!= (Variables|Default|GetCubeSelected) 0)
    _
    (else
      (bind _returnvalue (Game|SpawnActorfromClass (Variables|Default|GetPlayerCubeClass) (Transformation|GetActorTransform self) "Undefined" 0 0))
      (Variables|Default|SetCubeSelected _returnvalue)))
  (Utilities|FlowControl|Sequence
    (:then_0
      (EventDispatchers|AssignUpdateInventoryStateUpdate (Variables|/Script/Cube_TheBattleMaster.Player_Cube|GetAttachmentComponent (Variables|Default|GetCubeSelected)) (delegate Custom|UpdateInventoryStateUpdate_Event_0)))
    (:then_1
      (Utilities|IsValid (Variables|Default|GetAttachComponenets_UI)
        (:Is%20Valid
          (Default|UpdateData (Variables|Default|GetAttachComponenets_UI))
          (UserInterface|Viewport|AddtoViewport (Variables|Default|GetAttachComponenets_UI) 0))
        (:Is%20Not%20Valid
          (bind _returnvalue_2 (UserInterface|CreateWidget "/Game/MainMenu/AttachToCube/AttachWeaponsInterface.AttachWeaponsInterface_C"))
          (bind _output_get (Variables|Default|SetAttachComponenets_UI _returnvalue_2))
          (Default|SetInvRef _output_get (Variables|/Script/Cube_TheBattleMaster.Player_Cube|GetAttachmentComponent (Variables|Default|GetCubeSelected)))
          (UserInterface|Viewport|AddtoViewport _output_get 0)
          (Default|UpdateData _output_get)
          (Variables|/Game/MainMenu/AttachToCube/AttachWeaponsInterface.AttachWeaponsInterface_C|SetDummyCube _output_get (Variables|Default|GetCubeSelected)))))))

(event Custom|ED_Waiting_Event
  (bind _waitingwidget (Variables|Default|GetWaitingWidget))
  (if (Pawn|IsLocallyControlled)
    (Utilities|FlowControl|FlipFlop
      (:A
        (Widget|SetVisibility _waitingwidget "Visible"))
      (:B
        (Widget|SetVisibility _waitingwidget "Hidden")))))

(event Custom|Client_UpdateActions
  (params (Action%20UI :type Action%20Interface%20Object%20Reference) (MyPawn :type BP%20Pawn%20Object%20Reference))
  (Default|AddActiontoList Action%20UI MyPawn))

(event Custom|MC_UpdateActions
  (params (Action%20UI :type Action%20Interface%20Object%20Reference) (MyPawn :type BP%20Pawn%20Object%20Reference))
  (Networking|SwitchHasAuthority
    (:Authority
      (CallFunction|ClientUpdateActions Action%20UI MyPawn))
    (:Remote
      (CallFunction|ServerUpdateActions Action%20UI MyPawn))))

(event Custom|SetCubeClass
  (params (PlayerCubeClass :type Player%20Cube%20Class%20Reference))
  (bind _cubeselected (Variables|Default|GetCubeSelected))
  (bind _returnvalue (Utilities|GetClass _cubeselected))
  ;[1 1 1] For Setting the selected cube class on the server
  (Development|PrintString (Utilities|GetClassDisplayName PlayerCubeClass))
  (Development|PrintString (Utilities|GetClassDisplayName _returnvalue))
  (Networking|SwitchHasAuthority
    (:Authority
      (CallFunction|MulticastSetCubeClass _returnvalue))
    (:Remote
      (CallFunction|ServerSetCubeClass _returnvalue))))

(event Custom|Server_UpdateActions
  (params (Actions%20UI :type Action%20Interface%20Object%20Reference) (MyPawn :type BP%20Pawn%20Object%20Reference))
  (Default|AddActiontoList Actions%20UI MyPawn))

(event Custom|Server_ChangeMaterialCube
  (params (Material :type Material%20Interface%20Object%20Reference))
  ;[1 1 1] For changing cube material in the character slelection screen
  (CallFunction|MulticastMaterialCube Material))

(event Custom|Server_SpawnAttachItem
  ;[1 1 1] Temporary Spawnning items
  (bind _returnvalue (Game|SpawnActorfromClass (Utilities|Select :Index 3 :Option%200 "/Script/Cube_TheBattleMaster.Laser" :Option%201 "/Script/Cube_TheBattleMaster.Shield_Basic" :Option%202 "/Script/Cube_TheBattleMaster.BuildObject_Basic" :Option%203 "/Script/Cube_TheBattleMaster.Launcher_Basic" :Option%204 "/Script/Cube_TheBattleMaster.Booster_Basic") (Math|Transform|MakeTransform "0, 0, 0") "Undefined" self 0))
  (bind _asitem_base (Utilities|Casting|CastToItemBase _returnvalue))
  (CallFunction|AttachmentEquipInterface (Variables|Default|GetMyCube) _asitem_base (Utilities|Select :Index (Math|Random|RandomIntegerinRange 0 5) :Option%200 "S_Side1" :Option%201 "S_Side2" :Option%202 "S_Side3" :Option%203 "S_Side4" :Option%204 "S_Side5" :Option%205 "S_Side6")))

(event Custom|Multicast_SetCubeSave
  (params (SavedDetails :type My%20Save%20Game%20Object%20Reference))
  ;[1 1 1] Set cube save file
  (Variables|Default|SetImportedSavedDetails SavedDetails)
  (Development|PrintString (Utilities|GetDisplayName SavedDetails)))

(event Custom|Server_SetCubeSave
  (params (SavedDetails :type My%20Save%20Game%20Object%20Reference))
  ;[1 1 1] Set cube save file
)

(event Custom|TestForNow
  ;[1 1 1] Temporary Spawnning items
  (Class|CubetheBattleMasterPawn|UpdateActions))

(event Custom|SetCubeSave
  (params (SavedDetails :type My%20Save%20Game%20Object%20Reference))
  ;[1 1 1] Set cube save file
  (Development|PrintString (Utilities|GetDisplayName SavedDetails))
  (Networking|SwitchHasAuthority
    (:Remote
      (CallFunction|MulticastSetCubeSave SavedDetails))))

(event Custom|Server_SetCubeClass
  (params (PLayerCubeClass :type Player%20Cube%20Class%20Reference))
  ;[1 1 1] For Setting the selected cube class on the server
  (CallFunction|MulticastSetCubeClass PLayerCubeClass))

(event Custom|TogglleCamera
  (bind _outactors (Actor|GetAllActorsOfClass "/Script/Engine.CameraActor"))
  (bind (_array_element _array_index) (Utilities|Array|ForEachLoopwithBreak _outactors :!label _label)
    (:LoopBody
      (if (== _array_index (Variables|Default|GettoggleCamera))
        (Game|Player|SetViewTargetwithBlend (.AsPlayer%20Controller (Utilities|Casting|CastToPlayerController (Components|GetOwner))) _array_element 0.0 "VTBlend_Linear" 0.0 false)
        (Math|Integer|IncrementInt (Variables|Default|GettoggleCamera)
          (:%20%20
            (if (>= (Utilities|Array|Length _outactors) (Variables|Default|GettoggleCamera))
              (Variables|Default|SettoggleCamera 0)
              (goto _label Break)
              (else
                (goto _label Break)))))))))

(event Custom|Multicast_SetCubeClass
  (params (NewParam :type Player%20Cube%20Class%20Reference))
  ;[1 1 1] For Setting the selected cube class on the server
  (Variables|Default|SetPlayerCubeClass NewParam))

(event Custom|CharacterSelection
  (bind _self self)
  (bind _returnvalue (Components|GetOwner _self))
  (bind _asbp_player_controller (Utilities|Casting|CastToBP_PlayerController _returnvalue))
  (if (Pawn|IsLocallyControlled)
    (bind _returnvalue_2 (UserInterface|CreateWidget "/Game/MainMenu/CharacterSelection.CharacterSelection_C" _asbp_player_controller))
    (UserInterface|Viewport|AddtoViewport _returnvalue_2 0)
    (bind _returnvalue_3 (UserInterface|CreateWidget "/Game/MainMenu/WaitingWidget.WaitingWidget_C" _asbp_player_controller))
    (bind _output_get (Variables|Default|SetWaitingWidget _returnvalue_3))
    (Widget|SetVisibility _output_get "Hidden")
    (UserInterface|Viewport|AddtoViewport _output_get 0)))

(event Custom|ChangeMaterialCube
  (params (Material :type Material%20Interface%20Object%20Reference))
  ;[1 1 1] For changing cube material in the character slelection screen
  (Networking|SwitchHasAuthority
    (:Authority
      (CallFunction|MulticastMaterialCube))
    (:Remote
      (CallFunction|ServerChangeMaterialCube))))

(event Custom|Multicast_MaterialCube
  (params (Material :type Material%20Interface%20Object%20Reference))
  (bind _cubeselected (Variables|Default|GetCubeSelected))
  ;[1 1 1] For changing cube material in the character slelection screen
  (if (!= 0 _cubeselected)
    (Rendering|Material|SetMaterial (Variables|/Script/Cube_TheBattleMaster.Player_Cube|GetBlockMesh _cubeselected) 0 Material)
    (else
      (Networking|SwitchHasAuthority
        (:Authority
          (CallFunction|MulticastMaterialCube))
        (:Remote
          (CallFunction|ServerChangeMaterialCube))))))

(event Custom|UpdateInventoryStateUpdate_Event_0
  (bind _attachcomponenets_ui (Variables|Default|GetAttachComponenets_UI))
  (Default|UpdateData _attachcomponenets_ui)
  (UserInterface|Viewport|AddtoViewport _attachcomponenets_ui 0))

(event Custom|AttachItems_UI
  (Utilities|IsValid (Variables|Default|GetAttachComponenets_UI)
    (:Is%20Valid
      (UserInterface|Viewport|AddtoViewport (Variables|Default|GetAttachComponenets_UI) 0))
    (:Is%20Not%20Valid
      (bind _returnvalue (UserInterface|CreateWidget "/Game/MainMenu/AttachToCube/AttachWeaponsInterface.AttachWeaponsInterface_C"))
      (bind _output_get (Variables|Default|SetAttachComponenets_UI _returnvalue))
      (UserInterface|Viewport|AddtoViewport _output_get 0))))

(event Custom|Client_SpawnAttachItem
  ;[1 1 1] Temporary Spawnning items
  (CallFunction|ServerSpawnAttachItem))

(event EventRefreshMovement
  (bind _personal_action_interface (Variables|Default|GetPersonal%20Action%20interface))
  (if (!= 0 _personal_action_interface)
    (Default|RefreshMovementListEventEvent _personal_action_interface)))

(event EventTick
  (params (DeltaSeconds :type Float%20%28single-precision%29))
  ;[1 1 1] MousePosition
  (bind _returnvalue (Class|WidgetLayoutLibrary|GetMousePositiononViewport))
  (Collision|LineTraceByChannel (.WorldPosition (Class|GameplayStatics|DeprojectScreentoWorld (Game|GetPlayerController 0) (* _returnvalue (Class|WidgetLayoutLibrary|GetViewportScale)))) (+ (* (.WorldDirection (Class|GameplayStatics|DeprojectScreentoWorld (Game|GetPlayerController 0) (* _returnvalue (Class|WidgetLayoutLibrary|GetViewportScale)))) 3e+03) (.WorldPosition (Class|GameplayStatics|DeprojectScreentoWorld (Game|GetPlayerController 0) (* _returnvalue (Class|WidgetLayoutLibrary|GetViewportScale))))) "TraceTypeQuery1" false 0 "None"))

(event EventCubeMaterialUpdate
  ;[1 1 1] For changing cube material in the character slelection screen
  (Utilities|FlowControl|Sequence
    (:then_0
      _)
    (:then_1
      _))
  (CallFunction|MulticastMaterialCube (stale Custom|Server_ChangeMaterialCube Material)))

(event EventRefreshEnergy
  (bind _ui_overlay (Variables|Default|GetUI_Overlay))
  (if (!= 0 _ui_overlay)
    (Default|RefreshEvent _ui_overlay)))

(event EventConfirmationButtonActive
  (params (bOn :type Boolean))
  (Default|ConfirmButtonEventEvent (Variables|Default|GetPersonal%20Action%20interface) bOn))

(event EventUpdateActions
  (bind _personal_action_interface (Variables|Default|GetPersonal%20Action%20interface))
  (|CallParentFunction)
  (if (!= 0 _personal_action_interface)
    (Default|RefreshActionButtonListEvent _personal_action_interface)))

(event EventBeginPlay)

(event EventActionSelected
  (|CallParentFunction)
  (Default|RefreshActionArrayEvent (Variables|Default|GetPersonal%20Action%20interface)))

(event EventResetButtonsTest
  (bind _ui_overlay (Variables|Default|GetUI_Overlay))
  (bind _personal_action_interface (Variables|Default|GetPersonal%20Action%20interface))
  (if (not (== 0 _personal_action_interface))
    (Default|ResettheButtonsEvent _personal_action_interface)
    (Default|RefreshActionArrayEvent _personal_action_interface)
    (if (!= 0 _ui_overlay)
      (Default|RefreshEvent _ui_overlay))))

(event EventCubeMade
  (Utilities|FlowControl|Sequence
    (:then_0
      (if (Pawn|IsLocallyControlled)
        (Utilities|FlowControl|Sequence
          (:then_0
            (bind _returnvalue (UserInterface|CreateWidget "/Game/Widgets/ActionsInterface/ActionInterface.ActionInterface_C"))
            (bind _output_get (Variables|Default|SetPersonal%20Action%20interface _returnvalue))
            (UserInterface|Viewport|AddtoViewport _output_get 0))
          (:then_1
            (bind _returnvalue_2 (UserInterface|CreateWidget "/Game/Widgets/ActionsInterface/ForWeaponsAndEnergy/AmunitionAndEnergy.AmunitionAndEnergy_C"))
            (bind _output_get_2 (Variables|Default|SetUI_Overlay _returnvalue_2))
            (UserInterface|Viewport|AddtoViewport _output_get_2 0)
            (Default|RefreshEvent (Variables|Default|GetUI_Overlay))))))
    (:then_1
      (Class|CubetheBattleMasterPawn|UpdateActions))))

(event EventConfirmActions
  (bind _personal_action_interface (Variables|Default|GetPersonal%20Action%20interface))
  (|CallParentFunction)
  (Widget|SetVisibility (Variables|/Game/Widgets/ActionsInterface/ActionInterface.ActionInterface_C|GetReady_Button _personal_action_interface) "Visible")
  (Widget|SetVisibility (Variables|/Game/Widgets/ActionsInterface/ActionInterface.ActionInterface_C|GetCancelButton _personal_action_interface) "Visible")
  (Widget|SetVisibility (Variables|/Game/Widgets/ActionsInterface/ActionInterface.ActionInterface_C|GetAttack_Button _personal_action_interface) "Hidden")
  (Widget|SetVisibility (Variables|/Game/Widgets/ActionsInterface/ActionInterface.ActionInterface_C|GetMove_Button _personal_action_interface) "Hidden")
  (Widget|SetVisibility (Variables|/Game/Widgets/ActionsInterface/ActionInterface.ActionInterface_C|GetActionButtonList _personal_action_interface) "Hidden")
  (Default|RefreshEvent (Variables|Default|GetUI_Overlay)))

(event EventCancelButton
  (bind _personal_action_interface (Variables|Default|GetPersonal%20Action%20interface))
  (|CallParentFunction)
  (Widget|SetVisibility (Variables|/Game/Widgets/ActionsInterface/ActionInterface.ActionInterface_C|GetReady_Button _personal_action_interface) "Hidden")
  (Widget|SetVisibility (Variables|/Game/Widgets/ActionsInterface/ActionInterface.ActionInterface_C|GetCancelButton _personal_action_interface) "Hidden")
  (Widget|SetVisibility (Variables|/Game/Widgets/ActionsInterface/ActionInterface.ActionInterface_C|GetAttack_Button _personal_action_interface) "Visible")
  (Widget|SetVisibility (Variables|/Game/Widgets/ActionsInterface/ActionInterface.ActionInterface_C|GetMove_Button _personal_action_interface) "Visible")
  (Widget|SetVisibility (Variables|/Game/Widgets/ActionsInterface/ActionInterface.ActionInterface_C|GetActionButtonList _personal_action_interface) "Visible")
  (Default|RefreshEvent (Variables|Default|GetUI_Overlay)))

(event EventReadyButton
  (bind _personal_action_interface (Variables|Default|GetPersonal%20Action%20interface))
  (|CallParentFunction)
  (Widget|SetVisibility (Variables|Default|GetPersonal%20Action%20interface) "Hidden")
  (Widget|SetVisibility (Variables|/Game/Widgets/ActionsInterface/ActionInterface.ActionInterface_C|GetReady_Button _personal_action_interface) "Hidden")
  (Widget|SetVisibility (Variables|/Game/Widgets/ActionsInterface/ActionInterface.ActionInterface_C|GetCancelButton _personal_action_interface) "Hidden")
  (Widget|SetVisibility (Variables|/Game/Widgets/ActionsInterface/ActionInterface.ActionInterface_C|GetAttack_Button _personal_action_interface) "Visible")
  (Widget|SetVisibility (Variables|/Game/Widgets/ActionsInterface/ActionInterface.ActionInterface_C|GetMove_Button _personal_action_interface) "Visible")
  (Widget|SetVisibility (Variables|/Game/Widgets/ActionsInterface/ActionInterface.ActionInterface_C|GetActionButtonList _personal_action_interface) "Visible")
  (Default|RefreshEvent (Variables|Default|GetUI_Overlay)))

(event EventWaiting
  (bind _waitingwidget (Variables|Default|GetWaitingWidget))
  (EventDispatchers|BindEventtoEDWaiting (delegate Custom|ED_Waiting_Event))
  (if (Pawn|IsLocallyControlled)
    (Utilities|FlowControl|FlipFlop
      (:A
        (Widget|SetVisibility _waitingwidget "Visible"))
      (:B
        (Widget|SetVisibility _waitingwidget "Hidden")))))

(event Input|KeyboardEvents|Backspace
  (params (Key :type Key%20Structure :default "None"))
  ;[1 1 1] Temporary Spawnning items
)

(event Input|KeyboardEvents|SpaceBar
  (params (Key :type Key%20Structure :default "None"))
  ;[1 1 1] Temporary Spawnning items
  (:Pressed
    (Default|RefreshEvent (Variables|Default|GetUI_Overlay))
    (Class|CubetheBattleMasterPawn|UpdateActions)))

(event Input|KeyboardEvents|Q
  (params (Key :type Key%20Structure :default "None"))
  (:Pressed
    (Class|CubetheBattleMasterPawn|Test)))

(event Input|KeyboardEvents|Backspace
  (params (Key :type Key%20Structure :default "None"))
  ;[1 1 1] Temporary Spawnning items
)

(event Input|KeyboardEvents|E
  (params (Key :type Key%20Structure :default "None"))
  (bind _mycube (Variables|Default|GetMyCube))
  (bind _returnvalue (Transformation|GetActorRotation _mycube))
  (bind (_roll _pitch _yaw) (Math|Rotator|BreakRotator _returnvalue))
  (:Pressed
    (if (!= _mycube 0)
      (Transformation|SetActorRelativeRotation _mycube (Math|Rotator|MakeRotator _roll _pitch (+ _yaw 9e+01))))))

(event Input|KeyboardEvents|Tab
  (params (Key :type Key%20Structure :default "None"))
  (:Pressed
    (bind _outactors (Actor|GetAllActorsOfClass "/Script/Engine.CameraActor"))
    (bind (_array_element _array_index) (Utilities|Array|ForEachLoopwithBreak _outactors :!label _label)
      (:LoopBody
        (if (== _array_index (Variables|Default|GettoggleCamera))
          (Game|Player|SetViewTargetwithBlend (.AsPlayer%20Controller (Utilities|Casting|CastToPlayerController (Components|GetOwner))) _array_element 0.0 "VTBlend_Linear" 0.0 false)
          (Math|Integer|IncrementInt (Variables|Default|GettoggleCamera)
            (:%20%20
              (if (>= (Utilities|Array|Length _outactors) (Variables|Default|GettoggleCamera))
                (Variables|Default|SettoggleCamera 0)
                (goto _label Break)
                (else
                  (goto _label Break))))))))))

(fn ConstructionScript)

(fn EDCubeSelectedSpawn
  (if (Pawn|IsLocalController (Pawn|GetController))
    (bind _returnvalue (Game|SpawnActorfromClass "/Script/Cube_TheBattleMaster.Player_Cube" (Math|Conversions|ToTransform(Vector) "0, 0, 0") "Undefined" 0 0))
    (Networking|SetReplicates _returnvalue false)
    (Development|PrintString (Utilities|String|Append (Utilities|GetDisplayName _returnvalue) (Utilities|GetDisplayName self)))
    (return _returnvalue)))

(fn SetCubeSelected
  (params (Location :type Vector :default "0, 0, 0"))
  (Class|ActorComponent|SetIsReplicated (Variables|Transformation|GetRootComponent) false)
  (return 0))

(fn AttachmentEquipInterface
  (params (Cube :type Player%20Cube%20Object%20Reference) (Item :type Item%20Base%20Object%20Reference) (SocketName :type Name))
  (Class|ItemBase|SetSlotName Item SocketName)
  (Class|ItemBase|Equip Item))